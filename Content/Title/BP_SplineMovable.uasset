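; Title-folder spline actor that moves a referenced skeletal mesh actor along its spline.
; BeginPlay calls Start, which enables Tick.
; While the target is valid, each tick advances a distance at a fixed speed and snaps the target to the spline's world position and rotation there, without sweep or scale.
; The distance has no wrap or end check.
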(event EventBeginPlay
  (CallFunction|Start))

(event Collision|EventActorBeginOverlap
  (params (OtherActor :type Actor%20Object%20Reference)))

(event EventTick
  (params (DeltaSeconds :type Float%20%28single-precision%29))
  (if (Utilities|IsValid (Variables|Default|GetSkeletalMeshComponent))
    (Variables|Default|SetDistance (+ (Variables|Default|GetDistance) (* DeltaSeconds 1e+03)))
    (Transformation|SetActorTransform (Variables|Default|GetSkeletalMeshComponent) (Spline|GetTransformatDistanceAlongSpline (Variables|Default|GetSpline) (+ (Variables|Default|GetDistance) (* DeltaSeconds 1e+03)) "World" false))))

(fn ConstructionScript)

(fn Start
  (Actor|Tick|SetActorTickEnabled true))