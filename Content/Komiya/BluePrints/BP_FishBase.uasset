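; Base fish that wanders inside the level's PhysicsVolume and can be shot down by actors tagged Bullet.
; Tick picks a random point in the volume's bounds, interpolates rotation toward it while moving forward, then picks another when close in 2D.
; Each bullet hit costs one HP; at zero it stops, activates Niagara, registers its second tag in BP_GameInstance's collection, then bursts and destroys itself after a delay.
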(event OnComponentBeginOverlap(FishCollison)
  (params (OverlappedComponent :type Primitive%20Component%20Object%20Reference) (OtherActor :type Actor%20Object%20Reference) (OtherComp :type Primitive%20Component%20Object%20Reference) (OtherBodyIndex :type Integer) (bFromSweep :type Boolean) (SweepResult :type Hit%20Result%20Structure%20%28by%20ref%29))
  (if (Actor|ActorHasTag OtherActor "Bullet")
    (Utilities|FlowControl|Sequence
      (:then_0
        (Actor|DestroyActor OtherActor))
      (:then_1
        (bind _result (Math|Integer|DecrementInt (Variables|Default|GetFishHp))
          (:%20%20
            (Variables|Default|SetFishHp _result)
            (if (<= (Variables|Default|GetFishHp) 0)
              (Variables|Default|SetisAlive false)
              (Components|Activation|Activate (Variables|Default|GetNiagara) false)
              (bind _asbp_game_instance (Utilities|Casting|CastToBP_GameInstance (Game|GetGameInstance)))
              (Default|RegistarCollection _asbp_game_instance (Utilities|Array|Get(acopy) (Variables|Actor|GetTags self) 1))
              (bind _values (Utilities|Map|Values (Variables|/Game/Komiya/BluePrints/BP_GameInstance.BP_GameInstance_C|GetCollection _asbp_game_instance)))
              (for _array_element _values
                (Utilities|FlowControl|Delay 7.0)
                (Niagara|SpawnSystematLocation "/Game/GGJ/_hamagami/Niagara/NS_WaterBurst.NS_WaterBurst" (Transformation|GetActorLocation))
                (Actor|DestroyActor)))))))))

(event EventBeginPlay
  (bind _returnvalue (Actor|GetActorOfClass "/Script/Engine.PhysicsVolume"))
  (Variables|Default|SetPhysicsVolume _returnvalue))

(event Collision|EventActorBeginOverlap
  (params (OtherActor :type Actor%20Object%20Reference)))

(event EventTick
  (params (DeltaSeconds :type Float%20%28single-precision%29))
  (if (Variables|Default|GetisAlive)
    (if (Variables|Default|GetisDecisionPlace)
      ;[1 1 1] 目的地を設定
      (CallFunction|DecisionPlace)
      (Variables|Default|SetisDecisionPlace false)
      (Utilities|FlowControl|DoOnce false
        (:Completed
          (Development|PrintString (Utilities|String|Append (Utilities|GetDisplayName self) (Utilities|String|ToString(Vector) (Variables|Default|GetRandom%20Location))))))
      (else
        (Utilities|FlowControl|Sequence
          (:then_0
            ;[1 1 1] 目的地の方向に回転
            (CallFunction|FishRotation)
            (if (<= (Class|KismetMathLibrary|DegAcos (Math|Vector|DotProduct (Math|Vector|GetForwardVector (Math|Rotator|MakeRotator 0.0 0.0 (.Yaw (Math|Rotator|BreakRotator (Transformation|GetActorRotation))))) (Math|Vector|GetForwardVector (Math|Rotator|MakeRotator 0.0 0.0 (.Yaw (Math|Rotator|BreakRotator (Math|Rotator|FindLookatRotation (Transformation|GetActorLocation) (Variables|Default|GetRandom%20Location)))))))) 5.0)
              (Variables|Default|SetisRotation false)))
          (:then_1
            ;[1 1 1] 目的地の方向に移動
            (if (Variables|Default|GetisMove)
              (CallFunction|FishMovement)
              (if (< (Math|Vector|Distance2D(Vector) (Variables|Default|GetRandom%20Location) (Transformation|GetActorLocation)) 1.5e+02)
                (Variables|Default|SetisDecisionPlace true)
                (Variables|Default|SetisMove true)))))))))

(fn ConstructionScript)

(fn FishMovement
  (Pawn|Input|AddMovementInput (Transformation|GetActorForwardVector) 1.0 false))

(fn FishRotation
  (Transformation|SetActorRotation (Math|Interpolation|RInterpTo (Transformation|GetWorldRotation (Variables|Default|GetArrow1)) (Math|Rotator|FindLookatRotation (Transformation|GetActorLocation) (Variables|Default|GetRandom%20Location)) (Utilities|Time|GetWorldDeltaSeconds) (Variables|Default|GetRotationSpeed))))

(fn DecisionPlace
  (bind _physicsvolume (Variables|Default|GetPhysicsVolume))
  (bind (_origin _boxextent) (Collision|GetActorBounds _physicsvolume false false))
  (Variables|Default|SetRandom%20Location (Math|Random|RandomPointinBoundingBox _origin _boxextent)))

(fn SetHp
  (params (Hp :type Integer))
  (Variables|Default|SetFishHp Hp))